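; Checkpoint actor that saves the player's location when an actor tagged EmeraldBullet overlaps it.
; Each trigger creates a new SaveInfo object, stores the player character's position rather than its own, writes it to the "Loc" slot and prints it.
; The Checkpoint flag only selects the billboard sprite, as both save branches are identical.
; The construction script applies that sprite and sizes the trigger box from ChangeHitbox.
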(event `self.ReceiveActorBeginOverlap`
  (params (OtherActor :type "Actor Object Reference"))
  (bind _saveinfo (`self.SaveInfo`))
  (bind (_returnvalue_x _returnvalue_y _returnvalue_z) (`KismetMathLibrary.BreakVector` (`self.K2_GetActorLocation` (`self.CharInfo`))))
  (bind (_returnvalue_x_2 _returnvalue_y_2 _returnvalue_z_2) (`KismetMathLibrary.BreakVector` (`self.K2_GetActorLocation` (`self.CharInfo`))))
  (if (`self.ActorHasTag` OtherActor "EmeraldBullet")
    (bind _returnvalue (`GameplayStatics.CreateSaveGameObject` "/Game/BlueprintClasses/Checkpoints/SaveInfo.SaveInfo_C"))
    (bind _assave_info (cast `/Game/BlueprintClasses/Checkpoints/SaveInfo` _returnvalue))
    (set `self.SaveInfo` _assave_info)
    (bind _as3dish_character (cast `/Game/ThirdPersonBP/Blueprints/3dishCharacter` (`GameplayStatics.GetPlayerCharacter` 0)))
    (set `self.CharInfo` _as3dish_character)
    (if (`self.Checkpoint`)
      (set `/Game/BlueprintClasses/Checkpoints/SaveInfo.CheckLocation` (`KismetMathLibrary.MakeVector` _returnvalue_x_2 _returnvalue_y_2 _returnvalue_z_2) (`self.SaveInfo`))
      (`GameplayStatics.SaveGameToSlot` _saveinfo "Loc")
      (else
        (set `/Game/BlueprintClasses/Checkpoints/SaveInfo.CheckLocation` (`KismetMathLibrary.MakeVector` _returnvalue_x _returnvalue_y _returnvalue_z) (`self.SaveInfo`))
        (`GameplayStatics.SaveGameToSlot` _saveinfo "Loc")))
    (`KismetSystemLibrary.PrintString` (`KismetStringLibrary.Conv_VectorToString` (`/Game/BlueprintClasses/Checkpoints/SaveInfo.CheckLocation` _saveinfo)))))

(fn `UserConstructionScript`
  (bind _billboard (`self.Billboard`))
  (`BoxComponent.SetBoxExtent` (`self.Box`) (`self.ChangeHitbox`) true)
  (if (`self.Checkpoint`)
    (`BillboardComponent.SetSprite` _billboard "/Game/BlueprintClasses/Checkpoints/Checkpoint.Checkpoint")
    (else
      (`BillboardComponent.SetSprite` _billboard "/Game/BlueprintClasses/Checkpoints/Green_Tick.Green_Tick"))))